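; BP_Interactionactor is an actor that runs a timed interaction with a widget progress display, destroying a referenced actor on completion.
; While Setinteraction is true, Tick accumulates time and passes the remaining fraction to its Interaction_GG widget through SetIntper.
; When time reaches Maxinteractiontime, it destroys Mosactor if valid.
; Otherwise it zeroes the timer and resets the "percent" material parameter directly on the Widget component.
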(event EventBeginPlay)

(event Collision|EventActorBeginOverlap
  (params (OtherActor :type Actor%20Object%20Reference)))

(event EventTick
  (params (DeltaSeconds :type Float%20%28single-precision%29))
  (bind _mosactor (Variables|Default|Getmosactor))
  (if (Variables|Default|Getsetinteraction)
    (Variables|Default|Setacc_time (+ (Variables|Default|Getacc_time) DeltaSeconds))
    (bind _asinteraction_gg (Utilities|Casting|CastToInteraction_GG (UserInterface|GetWidget (Variables|Default|GetWidget))))
    (Default|SetIntper _asinteraction_gg (- 1.0 (/ (Variables|Default|Getacc_time) (Variables|Default|Getmaxinteractiontime))))
    (if (>= (Variables|Default|Getacc_time) (Variables|Default|Getmaxinteractiontime))
      (Utilities|IsValid _mosactor
        (:Is%20Valid
          (Actor|DestroyActor _mosactor))))
    (else
      (Variables|Default|Setacc_time 0.0)
      (Rendering|Material|SetScalarParameterValueonMaterials (Variables|Default|GetWidget) "percent" 1.0))))

(fn ConstructionScript)