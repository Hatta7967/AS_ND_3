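; BP_MainHUD manages the game's main UI and settings screen widgets.
; On BeginPlay it creates Main_UI for player controller 0, adds it to the viewport and stores the reference.
; The Show_settingUI event lazily creates Setting__Ui, adding it to the viewport and focusing it on first use.
; Later calls reuse the cached widget and only set it visible, without refocusing it.
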(event Custom|Show_settingUI
  (Utilities|IsValid (Variables|Default|GetSetting_UI)
    (:Is%20Valid
      (Widget|SetVisibility (Variables|Default|GetSetting_UI) "Visible"))
    (:Is%20Not%20Valid
      (bind _returnvalue (UserInterface|CreateWidget "/Game/Blueprints/ND_UI/Setting__Ui.Setting__Ui_C"))
      (bind _output_get (Variables|Default|SetSetting_UI _returnvalue))
      (UserInterface|Viewport|AddtoViewport _output_get 0)
      (Widget|SetFocus (Variables|Default|GetSetting_UI)))))

(event EventBeginPlay
  (bind _returnvalue (UserInterface|CreateWidget "/Game/Blueprints/ND_UI/Main_UI.Main_UI_C" (Game|GetPlayerController 0)))
  ;[1 1 1] 뷰포트에 ui추가
  (UserInterface|Viewport|AddtoViewport _returnvalue 0)
  (Variables|Default|Setmain_UI _returnvalue))

(event Collision|EventActorBeginOverlap
  (params (OtherActor :type Actor%20Object%20Reference)))

(event EventTick
  (params (DeltaSeconds :type Float%20%28single-precision%29)))

(fn ConstructionScript)