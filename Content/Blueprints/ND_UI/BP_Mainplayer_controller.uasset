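; Main player controller that handles the settings menu and triggers data-driven spawning.
; On BeginPlay it adds the Enhanced Input mapping context and spawns a spawn manager at the world origin.
; The mode-change input requests the settings UI through the HUD, with paired events switching between paused UI-only and unpaused game-only modes.
; NumPad 1 passes the "Easy" row of the spawn table to the spawn manager.
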(event Custom|Show_setting_UI
  (bind _asbp_main_hud (Utilities|Casting|CastToBP_MainHUD (HUD|GetHUD)))
  (Default|ShowSettingUI _asbp_main_hud)
  (Input|SetInputModeUIOnly self 0 "DoNotLock" false)
  (Variables|Default|SetbShowMouseCursor true)
  (Game|SetGamePaused true))

(event Custom|Set_game_only_mod
  (Input|SetInputModeGameOnly self false)
  (Variables|Default|SetbShowMouseCursor false)
  (Game|SetGamePaused false))

(event Input|EnhancedActionEvents|EnhancedInputActionI_P_Modechange
  (params (ActionValue :type Boolean) (ElapsedSeconds :type Float%20%28double-precision%29) (TriggeredSeconds :type Float%20%28double-precision%29) (InputAction :type Input%20Action%20Object%20Reference :default "/Game/Blueprints/global/input/I_P_Modechange.I_P_Modechange"))
  (:Started
    (CallFunction|ShowSettingUI)))

(event EventBeginPlay
  (Input|AddMappingContext (PlayerController|LocalPlayerSubsystems|GetEnhancedInputLocalPlayerSubsystem self) "/Game/Blueprints/global/input/input_playercontroller.input_playercontroller" 0 "(bIgnoreAllPressedKeysUntilRelease=True,bForceImmediately=False,bNotifyUserSettings=False)")
  (bind _returnvalue (Game|SpawnActorfromClass "/Game/Blueprints/spawn_manager.spawn_manager_C" (Math|Transform|MakeTransform "0, 0, 0") "Undefined" "MultiplyWithRoot" 0 0))
  (Variables|Default|Setspawn _returnvalue))

(event EventTick
  (params (DeltaSeconds :type Float%20%28single-precision%29)))

(event Input|KeyboardEvents|NumPadOne
  (params (Key :type Key%20Structure :default "None"))
  (:Pressed
    (bind _returnvalue (Utilities|GetDataTableRow "/Game/01_Data/spawn_table.spawn_table" "Easy")
      (:then
        (Default|SpawnfromData (Variables|Default|Getspawn) _returnvalue)))))

(fn ConstructionScript)