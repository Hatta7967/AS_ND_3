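; Moves a static mesh back and forth in a straight line between its starting relative location and that of a target component.
; BeginPlay caches both endpoints and prints the start location.
; Each Tick compares distance travelled with segment length, swaps the endpoints once it is reached or passed, then steps the mesh along the normalized direction by Speed times delta time, without sweep.
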(event EventBeginPlay
  (bind _output_get (Variables|Default|SetStartLocation (Variables|/Script/Engine.SceneComponent|GetRelativeLocation (Variables|Default|GetStaticMesh))))
  (Development|PrintString (Utilities|String|ToString(Vector) _output_get))
  (Variables|Default|SetTargetLocation (Variables|/Script/Engine.SceneComponent|GetRelativeLocation (Variables|Default|GetTargetComponent))))

(event Collision|EventActorBeginOverlap
  (params (OtherActor :type Actor%20Object%20Reference)))

(event EventTick
  (params (DeltaSeconds :type Float%20%28single-precision%29))
  (Utilities|FlowControl|Sequence
    (:then_0
      ;[1 1 1] 가야할 거리
      (Variables|Default|Setlength (Math|Vector|VectorLength (- (Variables|Default|GetTargetLocation) (Variables|Default|GetStartLocation))))
      ;[1 1 1] 가고있는 거리
      (Variables|Default|Settravelled (Math|Vector|VectorLength (- (Variables|/Script/Engine.SceneComponent|GetRelativeLocation (Variables|Default|GetStaticMesh)) (Variables|Default|GetStartLocation)))))
    (:then_1
      ;[1 1 1] 위치 셔플 바꾸기
      (if (>= (Variables|Default|Gettravelled) (Variables|Default|Getlength))
        (Variables|Default|SetTempLocation (Variables|Default|GetStartLocation))
        (Variables|Default|SetStartLocation (Variables|Default|GetTargetLocation))
        (Variables|Default|SetTargetLocation (Variables|Default|GetTempLocation))))
    (:then_2
      ;[1 1 1] 이동
      (Transformation|SetRelativeLocation (Variables|Default|GetStaticMesh) (+ (Variables|/Script/Engine.SceneComponent|GetRelativeLocation (Variables|Default|GetStaticMesh)) (* (Math|Vector|Normalize (- (Variables|Default|GetTargetLocation) (Variables|Default|GetStartLocation))) (* (Variables|Default|Getspeed) DeltaSeconds))) false false))))

(fn ConstructionScript)